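; Annotation actor that shows a title and details text in the level through a BP_AnnotationWidget held by its AnnotationWidget component.
; Functions read and write both texts and toggle the details border between Visible and Hidden, printing its prior visibility.
; GetAnnotationData packs the Id, texts and actor transform into an Annotation struct, using the level name as Url and a camera transform from the player's pawn location and controller rotation.
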(fn `GetAnnotationData`
  (returns (Annotation :type "Annotation Structure"))
  (bind _asbp_annotation_widget (cast `/Game/BP_AnnotationWidget` (`WidgetComponent.GetWidget` (`self.Annotation Widget`))))
  (bind _returnvalue (`GameplayStatics.GetCurrentLevelName` true))
  (return (make `Annotation` (`self.Id`) _returnvalue (`KismetTextLibrary.Conv_TextToString` (`TextBlock.GetText` (`/Game/BP_AnnotationWidget.Title` _asbp_annotation_widget))) (`KismetTextLibrary.Conv_TextToString` (`MultiLineEditableTextBox.GetText` (`/Game/BP_AnnotationWidget.Details` _asbp_annotation_widget))) "" "" (`KismetMathLibrary.MakeTransform` (`self.K2_GetActorLocation` (`GameplayStatics.GetPlayerPawn` 0)) (`self.K2_GetActorRotation` (`GameplayStatics.GetPlayerController` 0))) (`self.GetTransform`))))

(fn `GetDetails`
  (returns (Details :type String))
  (bind _asbp_annotation_widget (cast `/Game/BP_AnnotationWidget` (`WidgetComponent.GetWidget` (`self.Annotation Widget`))))
  (return (`KismetTextLibrary.Conv_TextToString` (`MultiLineEditableTextBox.GetText` (`/Game/BP_AnnotationWidget.Details` _asbp_annotation_widget)))))

(fn `GetTitle`
  (returns (Details :type String))
  (bind _asbp_annotation_widget (cast `/Game/BP_AnnotationWidget` (`WidgetComponent.GetWidget` (`self.Annotation Widget`))))
  (return (`KismetTextLibrary.Conv_TextToString` (`TextBlock.GetText` (`/Game/BP_AnnotationWidget.Title` _asbp_annotation_widget)))))

(fn `SetDetails`
  (params (Details :type String))
  (bind _asbp_annotation_widget (cast `/Game/BP_AnnotationWidget` (`WidgetComponent.GetWidget` (`self.Annotation Widget`))))
  (`MultiLineEditableTextBox.SetText` (`/Game/BP_AnnotationWidget.Details` _asbp_annotation_widget) (`KismetTextLibrary.Conv_StringToText` Details))
  (return))

(fn `SetTitle`
  (params (Title :type String))
  (bind _asbp_annotation_widget (cast `/Game/BP_AnnotationWidget` (`WidgetComponent.GetWidget` (`self.Annotation Widget`))))
  (`TextBlock.SetText` (`/Game/BP_AnnotationWidget.Title` _asbp_annotation_widget) (`KismetTextLibrary.Conv_StringToText` Title))
  (return))

(fn `ToggleDetailsVisibility`
  (bind _asbp_annotation_widget (cast `/Game/BP_AnnotationWidget` (`WidgetComponent.GetWidget` (`self.Annotation Widget`))))
  (bind _detailsborder (`/Game/BP_AnnotationWidget.DetailsBorder` _asbp_annotation_widget))
  (bind _returnvalue (`Widget.GetVisibility` _detailsborder))
  (`KismetSystemLibrary.PrintString` (`|GetEnumeratorNameAsString` _returnvalue))
  (if (`|EnumEquality` _returnvalue "Visible")
    (`Widget.SetVisibility` _detailsborder "Hidden")
    (else
      (`Widget.SetVisibility` _detailsborder "Visible"))))

(fn `UserConstructionScript`)