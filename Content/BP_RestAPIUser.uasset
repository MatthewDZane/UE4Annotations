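; Actor that syncs BP_Annotation actors with a localhost annotation REST API through a RestAPITool object.
; On BeginPlay it requests annotations, and Tick polls until the response is ready, then spawns those whose URL matches the level name, attached to the PointCloud.
; The Save input posts new annotations (Id 0) or puts existing ones, destroys all, then re-fetches, using short fixed delays.
; Disconnected test calls for other endpoints remain in the graph.
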(event `self.ReceiveBeginPlay`
  (bind _returnvalue (`|GenericCreateObject` "/Script/Anthropology.RestAPITool" self))
  (set `RestAPITool.AnnotationAPIUrl` "http://localhost/annotations/index.php" _returnvalue)
  (bind _output_get (set `self.Annotation Rest API Caller` _returnvalue))
  (`RestAPITool.GetAnnotations` _output_get)
  (`KismetSystemLibrary.Delay` 0.2)
  (set `self.WaitingForAnnotations` true))

(event `self.ReceiveTick`
  (params (DeltaSeconds :type "Float (single-precision)"))
  (bind _returnvalue (`RestAPITool.GetResponseDataReady` (`self.Annotation Rest API Caller`)))
  (if (and _returnvalue (`self.WaitingForAnnotations`))
    (`self.LoadAnnotations`)
    (set `self.WaitingForAnnotations` false)
    (set `self.Saving` false)))

(event `InputAction|Save`
  (params (Key :type "Key Structure"))
  (:`Released`
    (if (`self.Saving`)
      (`KismetSystemLibrary.PrintString` "Still Performing Previous Save. Please wait.")
      (else
        (set `self.Saving` true)
        (`KismetSystemLibrary.PrintString` "Saving Annotations")
        (`self.SaveAnnotations`)
        (`KismetSystemLibrary.Delay` 0.2)
        (bind _outactors (`GameplayStatics.GetAllActorsOfClass` "/Game/BP_Annotation.BP_Annotation_C"))
        (for _array_element _outactors
          (`self.K2_DestroyActor` _array_element))
        (`RestAPITool.GetAnnotations` (`self.Annotation Rest API Caller`))
        (`KismetSystemLibrary.Delay` 0.2)
        (set `self.WaitingForAnnotations` true)))))

(fn `LoadAnnotations`
  (bind _returnvalue (`RestAPITool.GetResponseData` (`self.Annotation Rest API Caller`)))
  (for _array_element (break `Response` _returnvalue)
    (bind _returnvalue_2 (`GameplayStatics.GetCurrentLevelName` true))
    (if (`KismetStringLibrary.EqualEqual_StrStr` _returnvalue_2 (`.Url` (break `Annotation` _array_element)))
      (bind _returnvalue_3 (`|SpawnActorFromClass` "/Game/BP_Annotation.BP_Annotation_C" (`.Annotation_transform` (break `Annotation` _array_element)) "Undefined" "OverrideRootScale" null null))
      (bind _returnvalue_4 (`GameplayStatics.GetActorOfClass` "/Game/PointCloud.PointCloud_C"))
      (`self.K2_AttachToActor` _returnvalue_3 _returnvalue_4 "None" "KeepRelative" "KeepRelative" "KeepRelative" true)
      (set `/Game/BP_Annotation.Id` (break `Annotation` _array_element) _returnvalue_3)
      (`/Game/BP_Annotation.SetTitle` _returnvalue_3 (`.Title` (break `Annotation` _array_element)))
      (`/Game/BP_Annotation.SetDetails` _returnvalue_3 (`.Description` (break `Annotation` _array_element))))))

(fn `SaveAnnotations`
  (bind _annotation_rest_api_caller (`self.Annotation Rest API Caller`))
  (bind _outactors (`GameplayStatics.GetAllActorsOfClass` "/Game/BP_Annotation.BP_Annotation_C"))
  (for _array_element _outactors
    (bind _annotation (`/Game/BP_Annotation.GetAnnotationData` _array_element))
    (if (== (`/Game/BP_Annotation.Id` _array_element) 0)
      (`RestAPITool.PostAnnotation` _annotation_rest_api_caller _annotation)
      (`KismetSystemLibrary.PrintString` "Posting Annotation")
      (else
        (`RestAPITool.PutAnnotationById` _annotation_rest_api_caller _annotation)
        (`KismetSystemLibrary.PrintString` "Putting Annotation")))))

(fn `UserConstructionScript`)